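; Weapon actor, named as a thrown magazine, that runs a Niagara effect with a fixed bullet count and reads its particles back into Blueprint.
; On BeginPlay it passes itself to Niagara as the export callback object.
; ParticleData stores each particle position in Locations, prints the index, then destroys the actor.
; The sphere overlap and system-finished handlers are empty, and the damage calls are unwired.
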(event `self.ReceiveBeginPlay`
  (`NiagaraComponent.SetVariableInt` (`self.Niagara`) "BulletCOunt" 30)
  (`ActorComponent.Activate` (`self.Niagara`) false)
  (`NiagaraComponent.SetVariableObject` (`self.Niagara`) "Object" self)
  (add `NiagaraComponent.OnSystemFinished` (`self.Niagara`) (delegate `CustomEvent`)))

(event `CustomEvent`
  (params (PSystem :type "NiagaraComponent Object Reference")))

(event `self.ReceiveParticleData`
  (params (Data :type "Array of BasicParticleData Structure (by ref)") (NiagaraSystem :type "NiagaraSystem Object Reference") (SimulationPositionOffset :type "Vector Structure (by ref)"))
  (for _array_element Data
    (bind _returnvalue (`KismetArrayLibrary.Array_Add` (`self.Locations`) (`.Position` (break `BasicParticleData` _array_element))))
    (`KismetSystemLibrary.PrintString` (`KismetStringLibrary.Conv_IntToString` _returnvalue)))
  (`self.K2_DestroyActor`))

(event `self.Sphere.OnComponentBeginOverlap`
  (params (OverlappedComponent :type "PrimitiveComponent Object Reference") (OtherActor :type "Actor Object Reference") (OtherComp :type "PrimitiveComponent Object Reference") (OtherBodyIndex :type Integer) (bFromSweep :type Boolean) (SweepResult :type "HitResult Structure (by ref)")))

(fn `UserConstructionScript`)