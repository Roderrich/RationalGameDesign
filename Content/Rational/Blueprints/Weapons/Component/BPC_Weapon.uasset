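; Weapon component for the third-person character that handles firing, ammo, reloading and level-ups from a weapon data table.
; Shooting is gated by fire-rate and reload timers, then runs a debug-drawn capsule trace from the follow camera, auto-reloading on empty.
; Leveling up loads stats from the table row and sets the ability-unlocked flag.
; Hit damage and ability leveling are unimplemented, though ability row names are cached.
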(event `self.ReceiveBeginPlay`
  (bind _asbp_third_person_character (cast `/Game/ThirdPerson/Blueprints/BP_ThirdPersonCharacter` (`GameplayStatics.GetPlayerCharacter` 0)))
  (set `self.As BP Third Person Character` _asbp_third_person_character)
  (bind _outrownames (`DataTableFunctionLibrary.GetDataTableRowNames` (`self.WeaponDataTable`)))
  (set `self.Out Row Names Wep` _outrownames)
  (bind _outrownames_2 (`DataTableFunctionLibrary.GetDataTableRowNames` (`self.AbilityDataTable`)))
  (set `self.Out Row Names A` _outrownames_2))

(event `Shoot`
  (if (not (or (`KismetSystemLibrary.K2_IsValidTimerHandle` (`self.Shot Cooldown`)) (`KismetSystemLibrary.K2_IsValidTimerHandle` (`self.Reload Cooldown`))))
    (bind _returnvalue (`KismetSystemLibrary.K2_SetTimerDelegate` (delegate `FireCooldown`) (`self.FireRate`)))
    (set `self.Shot Cooldown` _returnvalue)
    (`self.HitScan`)))

(event `FireCooldown`
  (`KismetSystemLibrary.K2_ClearAndInvalidateTimerHandle` (`self.Shot Cooldown`)))

(event `StopShoot`)

(event `RefillAmmo`
  (if (not (`KismetSystemLibrary.K2_IsValidTimerHandle` (`self.Reload Cooldown`)))
    (bind _returnvalue (`KismetSystemLibrary.K2_SetTimerDelegate` (delegate `Refill`) (`self.ReloadS`)))
    (set `self.Reload Cooldown` _returnvalue)
    (message `/Game/Rational/Blueprints/BPI_Player.Reloading` (`self.As BP Third Person Character`) (`self.ReloadS`))))

(event `LevelUpWeapon`
  (bind _result (`/Engine/EditorBlueprintResources/StandardMacros.IncrementInt` (`self.Level`))
    (:`  `
      (bind _returnvalue (`|GetDataTableRow` (`self.WeaponDataTable`) (`|GetArrayItem` (`self.Out Row Names Wep`) (- _result 1)))
        (:`then`
          (`self.UpdateWepStats` _returnvalue)
          (set `self.AbilityUnlocked` true))))))

(event `Refill`
  (set `self.CurrentAmmo` (`self.MaxAmmo`))
  (`KismetSystemLibrary.K2_ClearAndInvalidateTimerHandle` (`self.Reload Cooldown`))
  (message `/Game/Rational/Blueprints/BPI_Player.Reloaded` (`self.As BP Third Person Character`)))

(event `LevelUpAbility`)

(event `HitScan`
  (bind _followcamera (`/Game/ThirdPerson/Blueprints/BP_ThirdPersonCharacter.FollowCamera` (`self.As BP Third Person Character`)))
  (bind _returnvalue (`SceneComponent.K2_GetComponentLocation` _followcamera))
  (if (not (== (`self.CurrentAmmo`) 0))
    (bind (_outhit _returnvalue_2) (`KismetSystemLibrary.CapsuleTraceSingle` :`Start` _returnvalue :`End` (+ _returnvalue (* (`SceneComponent.GetForwardVector` _followcamera) 10000.0)) :`Radius` 10.0 :`HalfHeight` 10.0 :`TraceChannel` "TraceTypeQuery1" :`DrawDebugType` "ForDuration" :`DrawTime` 15.0))
    (`/Engine/EditorBlueprintResources/StandardMacros.DecrementInt` (`self.CurrentAmmo`)
      (:`  `
        (if _returnvalue_2
          _
          (else
            _))
        (if (== (`self.CurrentAmmo`) 0)
          (`self.RefillAmmo`))))))

(fn `GetHit`
  (returns (Hit :type Boolean))
  (return (`self.Hit`)))

(fn `UpdateWepStats`
  (params (S_Weapons :type "/Game/Rational/Blueprints/Weapons/Data/Weapons/S_Weapons Structure (by ref)"))
  (bind (_level _damage _reloadtime _firerate _magazine _accuracy) (break `/Game/Rational/Blueprints/Weapons/Data/Weapons/S_Weapons` S_Weapons))
  (set `self.Level` _level)
  (set `self.Damage` _damage)
  (set `self.ReloadS` _reloadtime)
  (set `self.FireRate` _firerate)
  (bind _output_get (set `self.MaxAmmo` _magazine))
  (set `self.CurrentAmmo` _output_get)
  (set `self.Accuracy` _accuracy))