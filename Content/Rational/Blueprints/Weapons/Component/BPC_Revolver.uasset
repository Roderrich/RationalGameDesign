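; Revolver weapon component that loads base stats from DT_Revolver and Quick Draw ability stats per level from DT_AQuickDraw.
; HitScan fires camera-forward line traces that spend ammo, send damage to the hit actor and refill when empty.
; Once the ability is levelled, a shot at six rounds takes a separate ricochet branch, which so far only traces and prints, with no damage or bounce.
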(event `self.ReceiveBeginPlay`
  (`parent.ReceiveBeginPlay`)
  (set `self.AbilityDataTable` "/Game/Rational/Blueprints/Weapons/Data/Abilities/DT_AQuickDraw.DT_AQuickDraw")
  (bind _output_get (set `self.WeaponDataTable` "/Game/Rational/Blueprints/Weapons/Data/Weapons/DT_Revolver.DT_Revolver"))
  (bind _returnvalue (`|GetDataTableRow` _output_get "1")
    (:`then`
      (`self.UpdateWepStats` _returnvalue))))

(event `self.LevelUpAbility`
  (bind _result (`/Engine/EditorBlueprintResources/StandardMacros.IncrementInt` (`self.Ability Level`))
    (:`  `
      (bind _returnvalue (`|GetDataTableRow` (`self.AbilityDataTable`) (`KismetStringLibrary.Conv_StringToName` (`KismetStringLibrary.Conv_IntToString` _result)))
        (:`then`
          (`self.UpdateAbilityStats` _returnvalue))))))

(event `self.HitScan`
  (bind _followcamera (`/Game/ThirdPerson/Blueprints/BP_ThirdPersonCharacter.FollowCamera` (`self.As BP Third Person Character`)))
  (bind _returnvalue (`SceneComponent.K2_GetComponentLocation` _followcamera))
  (if (== (`self.Ability Level`) 0)
    (`self.NormalHitScan`)
    (`KismetSystemLibrary.PrintString` "Shot Revolver")
    (elif (== (`self.CurrentAmmo`) 6)
      (if (not (== (`self.CurrentAmmo`) 0))
        (bind (_outhit _returnvalue_2) (`KismetSystemLibrary.LineTraceSingle` :`Start` _returnvalue :`End` (+ _returnvalue (* (`SceneComponent.GetForwardVector` _followcamera) 10000.0)) :`TraceChannel` "TraceTypeQuery1" :`DrawDebugType` "ForDuration"))
        (`/Engine/EditorBlueprintResources/StandardMacros.DecrementInt` (`self.CurrentAmmo`)
          (:`  `
            (`KismetSystemLibrary.PrintString` "Richochet  Shot Revolver")
            (if _returnvalue_2
              _
              (else
                _))
            (if (== (`self.CurrentAmmo`) 0)
              (`self.RefillAmmo`)))))
      (else
        (`self.NormalHitScan`)
        (`KismetSystemLibrary.PrintString` " Ability Shot Revolver")))))

(fn `NormalHitScan`
  (bind _followcamera (`/Game/ThirdPerson/Blueprints/BP_ThirdPersonCharacter.FollowCamera` (`self.As BP Third Person Character`)))
  (bind _returnvalue (`SceneComponent.K2_GetComponentLocation` _followcamera))
  (if (not (== (`self.CurrentAmmo`) 0))
    (bind (_outhit _returnvalue_2) (`KismetSystemLibrary.LineTraceSingle` :`Start` _returnvalue :`End` (+ _returnvalue (* (`SceneComponent.GetForwardVector` _followcamera) 10000.0)) :`TraceChannel` "TraceTypeQuery1" :`DrawDebugType` "ForDuration"))
    (`/Engine/EditorBlueprintResources/StandardMacros.DecrementInt` (`self.CurrentAmmo`)
      (:`  `
        (`KismetSystemLibrary.PrintString` (`KismetStringLibrary.Conv_DoubleToString` (`self.Damage`)))
        (message `/Game/Rational/Blueprints/Enemies/BPI_Enemy.Damage` (`.HitActor` (`GameplayStatics.BreakHitResult` _outhit)) (`self.Damage`))
        (if _returnvalue_2
          _
          (else
            _))
        (if (== (`self.CurrentAmmo`) 0)
          (`self.RefillAmmo`))))))

(fn `UpdateAbilityStats`
  (params (S_Abilities :type "/Game/Rational/Blueprints/Weapons/Data/Abilities/S_Abilities Structure (by ref)"))
  (bind (_level _abilitystat1 _abilitystat2) (break `/Game/Rational/Blueprints/Weapons/Data/Abilities/S_Abilities` S_Abilities))
  (set `self.Ability Level` _level)
  (set `self.DamageMulti` _abilitystat1)
  (set `self.Richochet` _abilitystat2))