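; SMG weapon component that handles automatic hitscan fire, reloading and stats for a mag-throw ability.
; Shoot starts a looping timer at a fixed 420 rounds per minute, leaving FireRate unused, and StopShoot clears it.
; HitScan capsule-traces from the follow camera with debug drawing, sends damage and triggers a timed refill when empty.
; LevelUpAbility loads stats from DT_MagThrow; the throw itself is only an unused projectile-path prediction.
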(event `self.ReceiveBeginPlay`
  (set `self.WeaponDataTable` "/Game/Rational/Blueprints/Weapons/Data/Weapons/DT_SMG.DT_SMG")
  (set `self.AbilityDataTable` "/Game/Rational/Blueprints/Weapons/Data/Abilities/DT_MagThrow.DT_MagThrow")
  (`parent.ReceiveBeginPlay`))

(event `self.LevelUpAbility`
  (bind _result (`/Engine/EditorBlueprintResources/StandardMacros.IncrementInt` (`self.Ability Level`))
    (:`  `
      (bind _returnvalue (`|GetDataTableRow` (`self.AbilityDataTable`) (`KismetStringLibrary.Conv_StringToName` (`KismetStringLibrary.Conv_IntToString` _result)))
        (:`then`
          (`self.UpdateAbilityStats` _returnvalue)
          (set `self.Unlocked` true))))))

(event `self.Shoot`
  (bind _returnvalue (`KismetSystemLibrary.K2_SetTimerDelegate` (`|CreateDelegate` :!event `HitScan`) (/ 60.0 420.0) true))
  (set `self.AutomaticFireTimer` _returnvalue))

(event `self.RefillAmmo`
  (bind _returnvalue (`KismetSystemLibrary.K2_SetTimerDelegate` (delegate `self.Refill`) (`self.ReloadS`)))
  (set `self.Reload Cooldown` _returnvalue)
  (`GameplayStatics.Blueprint_PredictProjectilePath_ByTraceChannel` (0.0 0.0 0.0)))

(event `self.StopShoot`
  (`KismetSystemLibrary.K2_ClearAndInvalidateTimerHandle` (`self.AutomaticFireTimer`)))

(event `self.Refill`
  (set `self.CurrentAmmo` (`self.MaxAmmo`))
  (`KismetSystemLibrary.K2_ClearAndInvalidateTimerHandle` (`self.Reload Cooldown`)))

(event `self.HitScan`
  (bind _followcamera (`/Game/ThirdPerson/Blueprints/BP_ThirdPersonCharacter.FollowCamera` (`self.As BP Third Person Character`)))
  (bind _returnvalue (`SceneComponent.K2_GetComponentLocation` _followcamera))
  (if (not (== (`self.CurrentAmmo`) 0))
    (bind (_outhit _returnvalue_2) (`KismetSystemLibrary.CapsuleTraceSingle` :`Start` _returnvalue :`End` (+ _returnvalue (* (`SceneComponent.GetForwardVector` _followcamera) 10000.0)) :`Radius` 10.0 :`HalfHeight` 10.0 :`TraceChannel` "TraceTypeQuery1" :`DrawDebugType` "ForDuration" :`DrawTime` 15.0))
    (`/Engine/EditorBlueprintResources/StandardMacros.DecrementInt` (`self.CurrentAmmo`)
      (:`  `
        (message `/Game/Rational/Blueprints/Enemies/BPI_Enemy.Damage` (`.HitActor` (`GameplayStatics.BreakHitResult` _outhit)) (`self.Damage`))
        (if _returnvalue_2
          _
          (else
            _))
        (if (== (`self.CurrentAmmo`) 0)
          (`self.RefillAmmo`))))))

(fn `UpdateAbilityStats`
  (params (S_Abilities :type "/Game/Rational/Blueprints/Weapons/Data/Abilities/S_Abilities Structure (by ref)"))
  (bind (_level _abilitystat1 _abilitystat2 _abilitystat3) (break `/Game/Rational/Blueprints/Weapons/Data/Abilities/S_Abilities` S_Abilities))
  (set `self.Ability Level` _level)
  (set `self.MagDamage` _abilitystat1)
  (set `self.Fuse` _abilitystat2)
  (set `self.Radius` _abilitystat3))