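; Shotgun weapon component that fires ten camera-based sphere-trace pellets per shot, sending damage to hit actors and spawning a projectile toward each trace result.
; Normal shots scatter pellets in an accuracy cone and share damage between them.
; Once the DoubleTap ability is leveled, every ShotNum-th shot instead fires all pellets straight ahead at longer range with bonus damage per pellet.
; Ability levels load stats from a DataTable, and empty ammo triggers a refill.
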(event `self.ReceiveBeginPlay`
  (set `self.WeaponDataTable` "/Game/Rational/Blueprints/Weapons/Data/Weapons/DT_Shotgun.DT_Shotgun")
  (`parent.ReceiveBeginPlay`)
  (set `self.AbilityDataTable` "/Game/Rational/Blueprints/Weapons/Data/Abilities/DT_ADoubleTap.DT_ADoubleTap"))

(event `self.LevelUpAbility`
  (bind _result (`/Engine/EditorBlueprintResources/StandardMacros.IncrementInt` (`self.Ability Level`))
    (:`  `
      (bind _returnvalue (`|GetDataTableRow` (`self.AbilityDataTable`) (`KismetStringLibrary.Conv_StringToName` (`KismetStringLibrary.Conv_IntToString` _result)))
        (:`then`
          (`self.UpdateAbilityStats` _returnvalue))))))

(event `self.HitScan`
  (bind _followcamera (`/Game/ThirdPerson/Blueprints/BP_ThirdPersonCharacter.FollowCamera` (`self.As BP Third Person Character`)))
  (bind _returnvalue (`SceneComponent.K2_GetComponentLocation` _followcamera))
  (if (== (`self.Ability Level`) 0)
    (`self.NormalHitScan`)
    (elif (not (== (`self.CurrentAmmo`) 0))
      (bind _result (`/Engine/EditorBlueprintResources/StandardMacros.IncrementInt` (`self.CurrentShotNum`))
        (:`  `
          (if (== _result (`self.ShotNum`))
            (set `self.CurrentShotNum` 0)
            (if (not (== (`self.CurrentAmmo`) 0))
              (for _ (range 10)
                (bind (_outhit _returnvalue_2) (`KismetSystemLibrary.SphereTraceSingle` _returnvalue (+ _returnvalue (* (`SceneComponent.GetForwardVector` _followcamera) 10000.0)) 2.0 "TraceTypeQuery1"))
                (bind (_bblockinghit _binitialoverlap _time _distance _location _impactpoint _normal _impactnormal _physmat _hitactor _hitcomponent _hitbonename _bonename _hititem _elementindex _faceindex _tracestart _traceend) (`GameplayStatics.BreakHitResult` _outhit))
                (message `/Game/Rational/Blueprints/Enemies/BPI_Enemy.Damage` _hitactor (+ (/ (`self.Damage`) 10.0) (`self.DamageMulti`)))
                (if _returnvalue_2
                  (`self.Projectile` _impactpoint)
                  (else
                    (`self.Projectile` _traceend)))
                (if (== (`self.CurrentAmmo`) 0)
                  (`self.RefillAmmo`)))
              (`/Engine/EditorBlueprintResources/StandardMacros.DecrementInt` (`self.CurrentAmmo`)
                (:`  `
                  (if (== (`self.CurrentAmmo`) 0)
                    (`self.RefillAmmo`)))))
            (else
              (`self.NormalHitScan`))))))))

(event `/Game/Rational/Blueprints/Weapons/BPI_Weapon.UnlockWeapon`
  (set `self.WeaponUnlocked` true))

(fn `NormalHitScan`
  (bind _followcamera (`/Game/ThirdPerson/Blueprints/BP_ThirdPersonCharacter.FollowCamera` (`self.As BP Third Person Character`)))
  (bind _returnvalue (`SceneComponent.K2_GetComponentLocation` _followcamera))
  (if (not (== (`self.CurrentAmmo`) 0))
    (for _ (range 10)
      (bind (_outhit _returnvalue_2) (`KismetSystemLibrary.SphereTraceSingle` _returnvalue (+ _returnvalue (* (`KismetMathLibrary.RandomUnitVectorInConeInDegrees` (`SceneComponent.GetForwardVector` _followcamera) (`self.Accuracy`)) 1000.0)) 2.0 "TraceTypeQuery1"))
      (bind (_bblockinghit _binitialoverlap _time _distance _location _impactpoint _normal _impactnormal _physmat _hitactor _hitcomponent _hitbonename _bonename _hititem _elementindex _faceindex _tracestart _traceend) (`GameplayStatics.BreakHitResult` _outhit))
      (message `/Game/Rational/Blueprints/Enemies/BPI_Enemy.Damage` _hitactor (/ (`self.Damage`) 10.0))
      (if _returnvalue_2
        (`self.Projectile` _impactpoint)
        (else
          (`self.Projectile` _traceend)))
      (if (== (`self.CurrentAmmo`) 0)
        (`self.RefillAmmo`)))
    (`/Engine/EditorBlueprintResources/StandardMacros.DecrementInt` (`self.CurrentAmmo`)
      (:`  `
        (if (== (`self.CurrentAmmo`) 0)
          (`self.RefillAmmo`))))))

(fn `UpdateAbilityStats`
  (params (S_Abilities :type "/Game/Rational/Blueprints/Weapons/Data/Abilities/S_Abilities Structure (by ref)"))
  (bind (_level _abilitystat1 _abilitystat2) (break `/Game/Rational/Blueprints/Weapons/Data/Abilities/S_Abilities` S_Abilities))
  (set `self.Ability Level` _level)
  (set `self.DamageMulti` _abilitystat1)
  (set `self.ShotNum` _abilitystat2))