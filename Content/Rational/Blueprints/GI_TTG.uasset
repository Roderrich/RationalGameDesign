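; Game instance that unlocks the shotgun and SMG through quick kill streaks and persists the weapon upgrade pool.
; Init binds Check to enemy deaths and loads or creates the BP_SaveWeapons save.
; Check counts kills per locked weapon, with timers that zero each streak, then on unlock notifies the character's weapon component, extends the pool and saves.
; The SMG branch relies on the character reference fetched in the shotgun branch.
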(event `self.ReceiveInit`
  (add `self.EnemyDeath` (delegate `Check`))
  (bind _returnvalue (`GameplayStatics.DoesSaveGameExist` (`self.Slot Name`)))
  (if _returnvalue
    (bind _returnvalue_2 (`GameplayStatics.LoadGameFromSlot` (`self.Slot Name`)))
    (bind _asbp_save_weapons (cast `/Game/Rational/Blueprints/Save/BP_SaveWeapons` _returnvalue_2)
      (:`then`
        ; Change to struct with the booleans
        (bind _output_get (set `self.SaveObject` _asbp_save_weapons))
        (bind (_savedata_weapons _savedata_shotgununlock _savedata_smgunlock) (break `/Game/Rational/Blueprints/Save/S_Save` (`/Game/Rational/Blueprints/Save/BP_SaveWeapons.SaveData` _output_get)))
        (set `self.WepUpgradePool` _savedata_weapons)
        (set `self.ShotgunUnlocked` _savedata_shotgununlock)
        (set `self.SMGUnlocked` _savedata_smgunlock))
      (:`CastFailed`
        (`KismetSystemLibrary.PrintString` "cast faileedddd")))
    (else
      (bind _returnvalue_3 (`GameplayStatics.CreateSaveGameObject` "/Game/Rational/Blueprints/Save/BP_SaveWeapons.BP_SaveWeapons_C"))
      (set `self.SaveObject` _returnvalue_3))))

(event `Check`
  (`|ExecutionSequence`
    (:`then_0`
      (if (not (`self.ShotgunUnlocked`))
        (bind _player (message `/Game/Rational/Blueprints/BPI_Gamemode.GetPlayer` (`GameplayStatics.GetGameMode`)))
        (set `self.As BP Third Person Character` _player)
        (bind _result (`/Engine/EditorBlueprintResources/StandardMacros.IncrementInt` (`self.KillsforShotgun`))
          (:`  `
            (if (>= _result 2)
              ; Shotgun true Unlock
              (message `/Game/Rational/Blueprints/Weapons/BPI_Weapon.UnlockWeapon` (`/Game/ThirdPerson/Blueprints/BP_ThirdPersonCharacter.BPC_Shotgun` (`self.As BP Third Person Character`)))
              (`KismetArrayLibrary.Array_Add` (`self.WepUpgradePool`) "/Game/Rational/Blueprints/Weapons/Data/Weapons/DT_Shotgun.DT_Shotgun")
              (set `self.ShotgunUnlocked` true)
              (`KismetSystemLibrary.PrintString` "Shotgun Unlockedaaaaaaaaaaaaaaaa" true true (struct :`R` 1.0 :`G` 0.165844 :`A` 1.0) 123.0)
              (set `/Game/Rational/Blueprints/Save/BP_SaveWeapons.SaveData` (make `/Game/Rational/Blueprints/Save/S_Save` (`self.WepUpgradePool`) (`self.ShotgunUnlocked`) (`self.SMGUnlocked`)) (`self.SaveObject`))
              (`GameplayStatics.SaveGameToSlot` (`self.SaveObject`) (`self.Slot Name`))
              (else
                (`KismetSystemLibrary.K2_SetTimerDelegate` (delegate `ShotgunCount`) 7.0)))))))
    (:`then_1`
      (if (not (`self.SMGUnlocked`))
        (bind _result_2 (`/Engine/EditorBlueprintResources/StandardMacros.IncrementInt` (`self.KillsforSMG`))
          (:`  `
            (if (>= _result_2 10)
              (`/Game/Rational/Blueprints/Weapons/Component/BPC_Weapon.UnlockWeapon` (`/Game/ThirdPerson/Blueprints/BP_ThirdPersonCharacter.BPC_SMG` (`self.As BP Third Person Character`)))
              (`KismetArrayLibrary.Array_Add` (`self.WepUpgradePool`) "/Game/Rational/Blueprints/Weapons/Data/Weapons/DT_SMG.DT_SMG")
              (set `self.SMGUnlocked` true)
              (`KismetSystemLibrary.PrintString` "smgn Unlockedaaaaaaaaaaaaaaaa" true true (struct :`R` 1.0 :`G` 0.165844 :`A` 1.0) 123.0)
              (set `/Game/Rational/Blueprints/Save/BP_SaveWeapons.SaveData` (make `/Game/Rational/Blueprints/Save/S_Save` (`self.WepUpgradePool`) (`self.ShotgunUnlocked`) (`self.SMGUnlocked`)) (`self.SaveObject`))
              (`GameplayStatics.SaveGameToSlot` (`self.SaveObject`) (`self.Slot Name`))
              (else
                (`KismetSystemLibrary.K2_SetTimerDelegate` (delegate `SMGCount`) 5.0)))))))))

(event `ShotgunCount`
  (set `self.KillsforShotgun` 0)
  (`KismetSystemLibrary.PrintString` "Shotgun reset"))

(event `CustomEvent`
  (`self.EnemyDeath`))

(event `SMGCount`
  (set `self.KillsforSMG` 0)
  (`KismetSystemLibrary.PrintString` "SMG reset"))

(fn `GetWeapons`
  (returns (Weapons :type "Array of DataTable Object Reference"))
  (return (`self.WepUpgradePool`)))