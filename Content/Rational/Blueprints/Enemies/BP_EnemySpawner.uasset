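; Enemy spawn point that creates a BP_Enemy at its own transform and triggers the game mode's enemy count message.
; Spawning runs from an event bound on BeginPlay, whose Type and Count inputs go unused.
; A trigger box, scaled by TriggerScale in the construction script, tracks BP_ThirdPersonCharacter overlap in TooClose.
; PlayerTooClose exposes that flag, but the spawn event itself does not check it.
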(event `self.ReceiveBeginPlay`
  (add `self.SpawnEnemy` (delegate `Spawn`)))

(event `Spawn` :!signature `self.SpawnEnemy`
  (params (Type :type "/Game/Rational/Blueprints/Enemies/Enum_Enemy Enum" :default "NewEnumerator0") (Count :type Integer))
  (`|SpawnActorFromClass` "/Game/Rational/Blueprints/Enemies/BP_Enemy.BP_Enemy_C" (`self.GetTransform`) "Undefined" "MultiplyWithRoot" null null)
  (message `/Game/Rational/Blueprints/BPI_Gamemode.EnemyCount` (`GameplayStatics.GetGameMode`)))

(event `self.Box.OnComponentBeginOverlap`
  (params (OverlappedComponent :type "PrimitiveComponent Object Reference") (OtherActor :type "Actor Object Reference") (OtherComp :type "PrimitiveComponent Object Reference") (OtherBodyIndex :type Integer) (bFromSweep :type Boolean) (SweepResult :type "HitResult Structure (by ref)"))
  (cast `/Game/ThirdPerson/Blueprints/BP_ThirdPersonCharacter` OtherActor)
  (set `self.TooClose` true))

(event `self.Box.OnComponentEndOverlap`
  (params (OverlappedComponent :type "PrimitiveComponent Object Reference") (OtherActor :type "Actor Object Reference") (OtherComp :type "PrimitiveComponent Object Reference") (OtherBodyIndex :type Integer))
  (cast `/Game/ThirdPerson/Blueprints/BP_ThirdPersonCharacter` OtherActor)
  (set `self.TooClose` false))

(fn `PlayerTooClose`
  (returns (TooClose :type Boolean))
  (return (`self.TooClose`)))

(fn `UserConstructionScript`
  (`SceneComponent.SetWorldScale3D` (`self.Box`) (`self.TriggerScale`)))