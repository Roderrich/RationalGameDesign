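; BP_Boss is a boss enemy Blueprint that extends a parent enemy class and takes its stats from the DT_Sniper data table.
; On BeginPlay it sets its enum type and looks up the row named after its Level, passing any found row to UpdateEnemyStats.
; Its UpdateEnemyStats override runs the parent logic, then forces a fixed max walk speed on the character movement.
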(event `self.ReceiveBeginPlay`
  (`parent.ReceiveBeginPlay`)
  (set `self.Enum_Type` "NewEnumerator2")
  (bind _output_get (set `self.Stats` "/Game/Rational/Blueprints/Enemies/Data/DT_Sniper.DT_Sniper"))
  (bind _returnvalue (`|GetDataTableRow` _output_get (`KismetStringLibrary.Conv_StringToName` (`KismetStringLibrary.Conv_IntToString` (`self.Level`))))
    (:`then`
      (`self.UpdateEnemyStats` _returnvalue))))

(fn `UpdateEnemyStats`
  (params (S_Player :type "/Game/Rational/Blueprints/Enemies/Data/S_Enemies_Base Structure (by ref)"))
  (`parent.UpdateEnemyStats` S_Player)
  (set `CharacterMovementComponent.MaxWalkSpeed` 200.0 (`self.CharacterMovement`))
  (return))

(fn `UserConstructionScript`
  (`parent.UserConstructionScript`))