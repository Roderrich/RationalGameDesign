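; Enemy AI controller that runs the BT_Enemy behavior tree and gives it the player as a blackboard object.
; The behavior tree is started from the Construction Script, while the Possess event is empty.
; BeginPlay casts player character 0 to BP_ThirdPersonCharacter, stores it and writes it to the "Player" key, printing an error if the cast fails.
; AnyDamage only prints a debug message.
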(event `self.ReceivePossess`
  (params (PossessedPawn :type "Pawn Object Reference")))

(event `self.ReceiveBeginPlay`
  (bind _asbp_third_person_character (cast `/Game/ThirdPerson/Blueprints/BP_ThirdPersonCharacter` (`GameplayStatics.GetPlayerCharacter` 0))
    (:`then`
      (bind _output_get (set `self.As BP Third Person Character` _asbp_third_person_character))
      (`BlackboardComponent.SetValueAsObject` (`AIBlueprintHelperLibrary.GetBlackboard` null) "Player" _output_get))
    (:`CastFailed`
      (`KismetSystemLibrary.PrintString` "Player Failed to found" true true (struct :`G` 0.66 :`B` 1.0 :`A` 1.0) 10.0))))

(event `self.ReceiveAnyDamage`
  (params (Damage :type "Float (single-precision)") (DamageType :type "DamageType Object Reference") (InstigatedBy :type "Controller Object Reference") (DamageCauser :type "Actor Object Reference"))
  (`KismetSystemLibrary.PrintString` "OWW" true true (struct :`G` 0.66 :`B` 1.0 :`A` 1.0) 10.0))

(fn `UserConstructionScript`
  (`self.RunBehaviorTree` "/Game/Rational/Blueprints/Enemies/BT_Enemy.BT_Enemy"))