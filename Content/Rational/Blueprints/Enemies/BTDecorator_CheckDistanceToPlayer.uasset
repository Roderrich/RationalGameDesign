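; Behavior tree decorator that gates enemy AI branches on proximity to the player.
; It reads the Player actor from the blackboard and passes when the controlled pawn is within a fixed 500-unit straight-line distance of it.
; The cast result is used without a validity check, and the range is hardcoded rather than exposed as a property.
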(fn `PerformConditionCheckAI`
  (params (OwnerController :type "AIController Object Reference") (ControlledPawn :type "Pawn Object Reference"))
  (returns (ReturnValue :type Boolean))
  (return (<= (`KismetMathLibrary.VSize` (- (`Actor.K2_GetActorLocation` ControlledPawn) (`Actor.K2_GetActorLocation` (cast `Actor` (`BTFunctionLibrary.GetBlackboardValueAsObject` (`self.Player`)) :!pure true)))) 500.0)))