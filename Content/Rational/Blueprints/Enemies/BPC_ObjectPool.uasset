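; BPC_ObjectPool is an object pool for enemies that hands out existing BP_Enemy actors by type.
; On BeginPlay it caches every BP_Enemy in the level into PooledActors.
; SelectUnusedEnemy claims and returns the first pooled enemy of the requested type not marked InUse.
; EnemyDeath moves the actor to world origin but sets InUse to true, so it does not free that enemy for reuse.
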(event `self.ReceiveBeginPlay`
  (bind _outactors (`GameplayStatics.GetAllActorsOfClass` "/Game/Rational/Blueprints/Enemies/BP_Enemy.BP_Enemy_C"))
  (set `self.Pooled Actors` _outactors))

(event `Enemy Death`
  (params (Actor :type "/Game/Rational/Blueprints/Enemies/BP_Enemy Object Reference"))
  (`Actor.K2_SetActorLocation` Actor (0.0 0.0 0.0) false false)
  (set `/Game/Rational/Blueprints/Enemies/BP_Enemy.In Use` true Actor))

(fn `SelectUnusedEnemy`
  (params (`Enemy TYpe` :type "/Game/Rational/Blueprints/Enemies/Data/Enum_EnemyType Enum" :default "NewEnumerator0"))
  (returns (`Array Element` :type "/Game/Rational/Blueprints/Enemies/BP_Enemy Object Reference"))
  (for _array_element (`self.Pooled Actors`)
    (if (`|EnumEquality` (`/Game/Rational/Blueprints/Enemies/BP_Enemy.Enum_Type` _array_element) `Enemy TYpe`)
      (if (not (`/Game/Rational/Blueprints/Enemies/BP_Enemy.In Use` _array_element))
        (set `/Game/Rational/Blueprints/Enemies/BP_Enemy.In Use` true _array_element)
        (set `self.Array Element` _array_element)
        (break))))
  (`/Engine/EditorBlueprintResources/StandardMacros.IsValid` (`self.Array Element`)
    (:`Is Valid`
      (return (`self.Array Element`)))))