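; AI controller for the sniper enemy that runs BT_Enemy_Sniper on possess, though its construction script also calls BT_Enemy.
; It caches the player character on BeginPlay and writes it to the blackboard.
; AI perception updates line of sight, and a cancellable delayed timer clears the Player key after sight is lost.
; Events forward attacks to the pawn, toggle HasAttacked, and pick a random retreat point around the player.
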(event `self.ReceivePossess`
  (params (PossessedPawn :type "Pawn Object Reference"))
  (set `self.Possessed Pawn` PossessedPawn)
  (set `self.NewVar` (make `GenericTeamId` 1))
  (`self.RunBehaviorTree` "/Game/Rational/Blueprints/Enemies/BT_Enemy_Sniper.BT_Enemy_Sniper"))

(event `self.ReceiveBeginPlay`
  (bind _asbp_third_person_character (cast `/Game/ThirdPerson/Blueprints/BP_ThirdPersonCharacter` (`GameplayStatics.GetPlayerCharacter` 0))
    (:`then`
      (bind _output_get (set `self.As BP Third Person Character` _asbp_third_person_character))
      (`BlackboardComponent.SetValueAsObject` (`AIBlueprintHelperLibrary.GetBlackboard` null) "Player" _output_get))
    (:`CastFailed`
      (`KismetSystemLibrary.PrintString` "Player Failed to found" true true (struct :`G` 0.66 :`B` 1.0 :`A` 1.0) 10.0))))

(event `TESSTTTT`)

(event `self.AIPerception.OnTargetPerceptionUpdated`
  (params (Actor :type "Actor Object Reference") (Stimulus :type "AIStimulus Structure"))
  (if (== Actor (`self.As BP Third Person Character`))
    (set `self.Preceived Actor` Actor)
    (if (`.bSuccessfullySensed` (break `AIStimulus` Stimulus))
      (`KismetSystemLibrary.K2_ClearAndInvalidateTimerHandle` (`self.Lost Sight Timer`))
      (`BlackboardComponent.SetValueAsBool` (`AIBlueprintHelperLibrary.GetBlackboard` null) "HasLineOfSight" true)
      (`BlackboardComponent.SetValueAsObject` (`AIBlueprintHelperLibrary.GetBlackboard` null) "Player" (`self.Preceived Actor`))
      (else
        (bind _returnvalue (`KismetSystemLibrary.K2_SetTimerDelegate` (delegate `LostSight`) 8.0))
        (set `self.Lost Sight Timer` _returnvalue)
        (`BlackboardComponent.SetValueAsBool` (`AIBlueprintHelperLibrary.GetBlackboard` null) "HasLineOfSight" false)))))

(event `self.GetAttackToken`)

(event `LostSight`
  (`BlackboardComponent.SetValueAsObject` (`AIBlueprintHelperLibrary.GetBlackboard` null) "Player" null))

(event `self.Attack`
  (message `/Game/Rational/Blueprints/Enemies/BPI_Enemy.Attack` (`self.K2_GetPawn`))
  (`BlackboardComponent.SetValueAsBool` (`AIBlueprintHelperLibrary.GetBlackboard` null) "HasAttacked" true))

(event `self.HasAttacked`
  (`BlackboardComponent.SetValueAsBool` (`AIBlueprintHelperLibrary.GetBlackboard` null) "HasAttacked" false))

(event `self.RetreatLocation`
  (params (Location :type "Vector Structure"))
  (`BlackboardComponent.SetValueAsVector` (`AIBlueprintHelperLibrary.GetBlackboard` null) "Location" (+ (`self.K2_GetActorLocation` (`self.As BP Third Person Character`)) (* (`KismetMathLibrary.RandomUnitVector`) 500.0))))

(fn `UserConstructionScript`
  (`self.RunBehaviorTree` "/Game/Rational/Blueprints/Enemies/BT_Enemy.BT_Enemy"))